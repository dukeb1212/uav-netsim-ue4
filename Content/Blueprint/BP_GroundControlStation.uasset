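; Ground control station actor that publishes its configured missions to the Mission Planner subsystem on BeginPlay.
; Each BPMission entry's waypoint and start-location actors are flattened into transform data, alongside the mission name and images.
; The resulting plans replace the subsystem's MissionPlans.
; Waypoint location and rotation arrays use AddUnique and are never cleared between missions, so they accumulate across entries and drop duplicate values.
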(event EventBeginPlay
  (bind _returnvalue (Subsystems|GetMissionPlannerSubsystem))
  (for _array_element (Variables|Default|GetBP_Mission)
    (for _array_element_2 (.waypoints _array_element)
      (Utilities|Array|AddUnique (Variables|Default|GetMission%20Locations) (Transformation|GetActorLocation _array_element_2))
      (Utilities|Array|AddUnique (Variables|Default|GetMission%20Rotations) (Transformation|GetActorRotation _array_element_2)))
    (Utilities|Array|AddUnique (Variables|Default|GetMission) (Utilities|Struct|MakeMissionPlan (.missionname _array_element) (Variables|Default|GetMission%20Locations) (Variables|Default|GetMission%20Rotations) (.images _array_element) (Transformation|GetActorLocation (.startlocation _array_element)))))
  (Utilities|Array|Clear (Variables|/Script/UAVNetSim.MissionPlannerSubsystem|GetMissionPlans _returnvalue))
  (Variables|/Script/UAVNetSim.MissionPlannerSubsystem|SetMissionPlans _returnvalue (Variables|Default|GetMission)))

(event Collision|EventActorBeginOverlap
  (params (OtherActor :type Actor%20Object%20Reference)))

(event EventTick
  (params (DeltaSeconds :type Float%20%28single-precision%29)))

(fn ConstructionScript)